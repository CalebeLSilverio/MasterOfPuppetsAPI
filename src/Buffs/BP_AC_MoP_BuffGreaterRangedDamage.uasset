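; Buff component that raises the owning character's ranged damage by a configurable percentage.
; On start it merges an additive item modifier into the ranged damage stat, converting the percentage to a fraction, and on clear it adds the negated value to undo it.
; It supplies a formatted effect description and accepts any actor, as the humanoid NPC check in CanBeAddedTo is disconnected.
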(event `self.GameplayEffectToApplyOnBuffStart`
  (`ConanCharacter.AddFloatStatModifier` (`self.OwningCharacter`) "DamageModifierRanged" "Item" "Add" (/ (`KismetMathLibrary.Conv_IntToDouble` (`self.BuffStatByThisMuch`)) 100.0) "Merge"))

(event `self.GameplayEffectToApplyOnBuffCleared`
  (`ConanCharacter.AddFloatStatModifier` (`self.OwningCharacter`) "DamageModifierRanged" "Item" "Add" (* -1 (/ (`KismetMathLibrary.Conv_IntToDouble` (`self.BuffStatByThisMuch`)) 100.0)) "Merge"))

(fn `CanBeAddedTo`
  (params (ContextActor :type "ConanCharacter Object Reference"))
  (returns (Result :type Boolean))
  (return true))

(fn `GetEffectDescription`
  (returns (Description :type Text))
  (return (`|FormatText` "Ranged Damage Increased by {0}%" (`self.BuffStatByThisMuch`))))