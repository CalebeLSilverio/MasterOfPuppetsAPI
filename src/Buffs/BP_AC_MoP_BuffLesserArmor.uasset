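; Lesser armor buff component that raises the owning character's Armor stat by a percentage while active.
; On start it converts the configured percentage of full Armor into a flat value, stores it, and merges it as an additive Item modifier.
; On clear it merges the negated stored value to undo the boost.
; It can be added to any actor, as the humanoid NPC check is disconnected.
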(event `self.GameplayEffectToApplyOnBuffStart`
  (bind _owningcharacter (`self.OwningCharacter`))
  (bind _output_get (set `self.BuffValue` (/ (* (`self.BuffStatByThisMuch`) (`ConanCharacter.GetFloatStat` _owningcharacter "Armor" "Full")) 100.0)))
  (`ConanCharacter.AddFloatStatModifier` _owningcharacter "Armor" "Item" "Add" _output_get "Merge"))

(event `self.GameplayEffectToApplyOnBuffCleared`
  (`ConanCharacter.AddFloatStatModifier` (`self.OwningCharacter`) "Armor" "Item" "Add" (* -1 (`self.BuffValue`)) "Merge"))

(fn `CanBeAddedTo`
  (params (ContextActor :type "ConanCharacter Object Reference"))
  (returns (Result :type Boolean))
  (return true))

(fn `GetEffectDescription`
  (returns (Description :type Text))
  (return (`|FormatText` "Armor Increased by {0}%" (`self.BuffStatByThisMuch`))))