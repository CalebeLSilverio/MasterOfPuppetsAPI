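; Lesser Survival buff component that raises the owning character's Metabolism attribute by a percentage, shown to players as a Survival increase.
; On start it computes the bonus from the full Metabolism stat, stores it, and merges it as an additive Item modifier.
; On clear it adds the negated stored value to undo the bonus.
; CanBeAddedTo always returns true, leaving its humanoid NPC check disconnected.
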(event `self.GameplayEffectToApplyOnBuffStart`
  (bind _owningcharacter (`self.OwningCharacter`))
  (bind _output_get (set `self.BuffValue` (/ (* (`ConanCharacter.GetIntStat` _owningcharacter "AttributeMetabolism" "Full") (`self.BuffStatByThisMuch`)) 100)))
  (`ConanCharacter.AddIntStatModifier` _owningcharacter "AttributeMetabolism" "Item" "Add" _output_get "Merge"))

(event `self.GameplayEffectToApplyOnBuffCleared`
  (`ConanCharacter.AddIntStatModifier` (`self.OwningCharacter`) "AttributeMetabolism" "Item" "Add" (* (`self.BuffValue`) -1) "Merge"))

(fn `CanBeAddedTo`
  (params (ContextActor :type "ConanCharacter Object Reference"))
  (returns (Result :type Boolean))
  (return true))

(fn `GetEffectDescription`
  (returns (Description :type Text))
  (return (`|FormatText` "Survival Increased by {0}%" (`self.BuffStatByThisMuch`))))