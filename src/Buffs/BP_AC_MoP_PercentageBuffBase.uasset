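; Base buff component that raises one int or float stat of the owning character by a percentage while active.
; On start it computes the amount from the full stat, caches it, and merges it as an additive modifier; on clear it merges the negated amount.
; Special cases: max health also raises current health on apply, Armor includes bonus armor in its base, and Str/Agi bonus weapon damage takes the raw percentage.
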(event `self.GameplayEffectToApplyOnBuffStart`
  (if (`self.IsIntStatToBuff`)
    (`self.ApplyIntStatBuff`)
    (else
      (`self.ApplyFloatStatBuff`))))

(event `self.GameplayEffectToApplyOnBuffCleared`
  (if (`self.IsIntStatToBuff`)
    (`self.ClearIntStatBuff`)
    (else
      (`self.ClearFloatStatBuff`))))

(fn `ApplyFloatStatBuff`
  (bind _floatstattobuff (`self.FloatStatToBuff`))
  (bind _returnvalue (`ConanCharacter.GetStatHolder` (`self.OwningCharacter`)))
  (bind _returnvalue_2 (`StatHolder.GetFloatStat` _returnvalue (`self.FloatStatToBuff`) "Full"))
  (`/Game/Systems/BP_MacroGlobal.Or+Branch` (`|EnumEquality` _floatstattobuff "BonusStrWeaponDmg") (`|EnumEquality` _floatstattobuff "BonusAgiWeaponDmg")
    (:`True`
      (`StatHolder.AddFloatStatModifier` (`ConanCharacter.GetStatHolder` (`self.OwningCharacter`)) (`self.FloatStatToBuff`) "Buff" "Add" (`self.PercentageToBuff`) "Merge"))
    (:`False`
      (if (`|EnumEquality` (`self.FloatStatToBuff`) "Armor")
        (bind _bonusarmor (message `/Game/Systems/Interfaces/IsBaseBPCombatInterface.GetBonusArmor` (`self.OwningCharacter`)))
        (set `self.FloatBuffValue` (* (+ _bonusarmor _returnvalue_2) (`self.PercentageToBuff`)))
        (else
          (set `self.FloatBuffValue` (* _returnvalue_2 (`self.PercentageToBuff`)))))
      (`StatHolder.AddFloatStatModifier` _returnvalue (`self.FloatStatToBuff`) "Buff" "Add" (`self.FloatBuffValue`) "Merge"))))

(fn `ApplyIntStatBuff`
  (bind _returnvalue (`ConanCharacter.GetStatHolder` (`self.OwningCharacter`)))
  (bind _output_get (set `self.IntBuffValue` (`KismetMathLibrary.FFloor` (* (`StatHolder.GetIntStat` _returnvalue (`self.IntStatToBuff`) "Full") (`self.PercentageToBuff`)))))
  (bind _returnvalue_2 (`StatHolder.AddIntStatModifier` _returnvalue (`self.IntStatToBuff`) "Buff" "Add" _output_get "Merge"))
  (if (and _returnvalue_2 (`|EnumEquality` (`self.IntStatToBuff`) "HealthMax"))
    (`StatHolder.AddToIntStat` _returnvalue "HealthCurrent" (`self.IntBuffValue`))))

(fn `CanBeAddedTo`
  (params (ContextActor :type "ConanCharacter Object Reference"))
  (returns (Result :type Boolean))
  (return true))

(fn `ClearFloatStatBuff`
  (bind _floatstattobuff (`self.FloatStatToBuff`))
  (`/Game/Systems/BP_MacroGlobal.Or+Branch` (`|EnumEquality` _floatstattobuff "BonusStrWeaponDmg") (`|EnumEquality` _floatstattobuff "BonusAgiWeaponDmg")
    (:`True`
      (`StatHolder.AddFloatStatModifier` (`ConanCharacter.GetStatHolder` (`self.OwningCharacter`)) (`self.FloatStatToBuff`) "Buff" "Add" (* -1 (`self.PercentageToBuff`)) "Merge"))
    (:`False`
      (`StatHolder.AddFloatStatModifier` (`ConanCharacter.GetStatHolder` (`self.OwningCharacter`)) (`self.FloatStatToBuff`) "Buff" "Add" (* -1 (`self.FloatBuffValue`)) "Merge"))))

(fn `ClearIntStatBuff`
  (`StatHolder.AddIntStatModifier` (`ConanCharacter.GetStatHolder` (`self.OwningCharacter`)) (`self.IntStatToBuff`) "Buff" "Add" (* (`self.IntBuffValue`) -1) "Merge"))

(fn `GetEffectDescription`
  (returns (Description :type Text))
  (return (`self.Description`)))